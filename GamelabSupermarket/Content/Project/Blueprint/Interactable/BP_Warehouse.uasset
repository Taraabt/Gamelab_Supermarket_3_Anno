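; BP_Warehouse is an interactable warehouse that hands out products to the player character.
; On BeginPlay it tints its cube with the game instance color that matches its Index.
; Interact adds a product to BP_DefaultCharacter when Index is 0 and the interactor is the first player, provided fewer than three products are held.
; Any other warehouse or interactor pairing only prints "Enemy".
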(event EventBeginPlay
  (bind _asbp_game_instance (Utilities|Casting|CastToBP_GameInstance (Game|GetGameInstance)))
  (Rendering|Material|SetColorParameterValueonMaterials (Variables|Default|GetCube) "Color" (Math|Conversions|ToLinearColor(Color) (Utilities|Array|Get(acopy) (Variables|/Game/Project/Blueprint/Core/BP_GameInstance.BP_GameInstance_C|GetColor _asbp_game_instance) (Variables|Default|GetIndex)))))

(event EventInteract
  (params (Interactor :type Character%20Object%20Reference))
  (if (and (== (Variables|Default|GetIndex) 0) (== Interactor (Game|Player|GetPlayerPawn 0)))
    (bind _asbp_default_character (Utilities|Casting|CastToBP_DefaultCharacter Interactor))
    (if (< (Utilities|Array|Length (Variables|/Game/Project/Blueprint/Player/BP_DefaultCharacter.BP_DefaultCharacter_C|GetProductName _asbp_default_character)) 3)
      (Default|AddProduct _asbp_default_character))
    (else
      (Development|PrintString "Enemy"))))

(fn ConstructionScript)