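; Interactable product slot whose point light shows whether it is occupied and lets the player remove a product.
; On BeginPlay it binds to the player character's LightOn event, which sets IsOn and lights the passed slot in a given color.
; Interacting while on removes the last entries from the character's product arrays, moves this slot's Index from Choose back to IndexDisponibili, and switches the light off.
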(event Custom|LightOn
  (params (NewParam :type BP%20Slott%20Object%20Reference) (NewParam2 :type Color%20Structure))
  (bind _pointlight (Variables|BP_Slott_C|GetPointLight NewParam))
  (Variables|Default|SetIsOn true)
  (Rendering|Components|Light|SetIntensity _pointlight 5e+03)
  (Rendering|Components|Light|SetLightColor _pointlight (Math|Conversions|ToLinearColor(Color) NewParam2) true))

(event EventBeginPlay
  (bind _asbp_default_character (Utilities|Casting|CastToBP_DefaultCharacter (Game|Player|GetPlayerPawn 0)))
  (EventDispatchers|BindEventtoLighton _asbp_default_character (EventDispatchers|CreateEvent :!event Custom|LightOn))
  (Variables|Default|SetIsOn false)
  (Rendering|Components|Light|SetIntensity (Variables|Default|GetPointLight) 0.0))

(event EventInteract
  (params (Interactor :type Character%20Object%20Reference))
  (if (Variables|Default|GetIsOn)
    (bind _asbp_default_character (Utilities|Casting|CastToBP_DefaultCharacter Interactor))
    (if (>= (Utilities|Array|Length (Variables|/Game/Project/Blueprint/Player/BP_DefaultCharacter.BP_DefaultCharacter_C|GetProductName _asbp_default_character)) 0)
      (Utilities|Array|RemoveIndex (Variables|/Game/Project/Blueprint/Player/BP_DefaultCharacter.BP_DefaultCharacter_C|GetProductName _asbp_default_character) (- (Utilities|Array|Length (Variables|/Game/Project/Blueprint/Player/BP_DefaultCharacter.BP_DefaultCharacter_C|GetProductName _asbp_default_character)) 1))
      (Utilities|Array|RemoveIndex (Variables|/Game/Project/Blueprint/Player/BP_DefaultCharacter.BP_DefaultCharacter_C|GetProductSlot _asbp_default_character) (- (Utilities|Array|Length (Variables|/Game/Project/Blueprint/Player/BP_DefaultCharacter.BP_DefaultCharacter_C|GetProductName _asbp_default_character)) 1))
      (for _array_element (Variables|/Game/Project/Blueprint/Player/BP_DefaultCharacter.BP_DefaultCharacter_C|GetChoose _asbp_default_character)
        (if (== _array_element (Variables|Default|GetIndex))
          (Utilities|Array|Add (Variables|/Game/Project/Blueprint/Player/BP_DefaultCharacter.BP_DefaultCharacter_C|GetIndexDisponibili _asbp_default_character) _array_element)
          (Utilities|Array|RemoveItem (Variables|/Game/Project/Blueprint/Player/BP_DefaultCharacter.BP_DefaultCharacter_C|GetChoose _asbp_default_character) _array_element)))
      (if (Variables|Default|GetIsOn)
        (Development|PrintString (Utilities|String|ToString(Integer) (Utilities|Array|Length (Variables|/Game/Project/Blueprint/Player/BP_DefaultCharacter.BP_DefaultCharacter_C|GetProductName _asbp_default_character))))
        (Rendering|Components|Light|SetIntensity (Variables|Default|GetPointLight) 0.0)
        (Variables|Default|SetIsOn false)))))

(fn ConstructionScript)