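; Thunderbolt power-up that, on overlap, stuns every unshielded enemy and player character except the one who touched it.
; Stunning sets the stun flag and shows stars and lightning; enemies also get an AI blackboard flag and halted movement.
; The pickup hides and disables overlaps, then a timer runs DeStunAll.
; DeStunAll removes shields from shielded characters, including the collector, clears stun on the rest, then destroys the actor.
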(event Custom|DeStunAll
  (bind _outactors (Actor|GetAllActorsOfClass "/Script/Engine.Character"))
  (for _array_element _outactors
    (bind _asbp_enemy (Utilities|Casting|CastToBP_Enemy _array_element)
      (:then
        (if (Variables|/Game/Project/Blueprint/AI/BP_Enemy.BP_Enemy_C|GetHasShield _asbp_enemy)
          (Variables|/Game/Project/Blueprint/AI/BP_Enemy.BP_Enemy_C|SetHasShield _asbp_enemy false)
          (else
            (AI|Components|Blackboard|SetValueasBool (Variables|/Script/AIModule.AIController|GetBlackboard (AI|GetAIController _asbp_enemy)) (Variables|Default|GetKey%20Name) false)
            (Variables|/Game/Project/Blueprint/AI/BP_Enemy.BP_Enemy_C|SetIsStunned _asbp_enemy false)
            (Components|Activation|Deactivate (Variables|/Game/Project/Blueprint/AI/BP_Enemy.BP_Enemy_C|GetStars _asbp_enemy))
            (Rendering|SetVisibility (Variables|/Game/Project/Blueprint/AI/BP_Enemy.BP_Enemy_C|GetStars _asbp_enemy) false false))))
      (:CastFailed
        (bind _asbp_default_character (Utilities|Casting|CastToBP_DefaultCharacter _array_element))
        (if (Variables|/Game/Project/Blueprint/Player/BP_DefaultCharacter.BP_DefaultCharacter_C|GetHasShield _asbp_default_character)
          (Variables|/Game/Project/Blueprint/Player/BP_DefaultCharacter.BP_DefaultCharacter_C|SetHasShield _asbp_default_character false)
          (else
            (Variables|/Script/GamelabSupermarket.DefaultCharacter|SetbIsStunned _asbp_default_character false)
            (Components|Activation|Deactivate (Variables|/Game/Project/Blueprint/Player/BP_DefaultCharacter.BP_DefaultCharacter_C|GetStars _asbp_default_character))
            (Rendering|SetVisibility (Variables|/Game/Project/Blueprint/Player/BP_DefaultCharacter.BP_DefaultCharacter_C|GetStars _asbp_default_character) false false))))))
  (Actor|DestroyActor))

(event EventBeginPlay
  (|CallParentFunction) ; This node is disabled and will not be called.\nDrag off pins to build functionality.
)

(event Collision|EventActorBeginOverlap
  (params (OtherActor :type Actor%20Object%20Reference))
  (|CallParentFunction 0)
  (Rendering|SetVisibility (Variables|Default|GetNiagara) false false)
  (Audio|PlaySound2D "/Game/Project/Sound/SFX/PowerUPS/PWRUP_Zap_CUT.PWRUP_Zap_CUT" 1.0 1.0 0.0 0 0)
  (bind _outactors (Actor|GetAllActorsOfClass "/Script/Engine.Character"))
  (for _array_element _outactors
    (if (not (== _array_element OtherActor))
      (bind _asbp_enemy (Utilities|Casting|CastToBP_Enemy _array_element)
        (:then
          (if (not (Variables|/Game/Project/Blueprint/AI/BP_Enemy.BP_Enemy_C|GetHasShield _asbp_enemy))
            (AI|Components|Blackboard|SetValueasBool (Variables|/Script/AIModule.AIController|GetBlackboard (AI|GetAIController _asbp_enemy)) (Variables|Default|GetKey%20Name) true)
            (Variables|/Game/Project/Blueprint/AI/BP_Enemy.BP_Enemy_C|SetIsStunned _asbp_enemy true)
            (Components|Movement|StopMovementImmediately (Variables|/Script/Engine.Character|GetCharacterMovement _asbp_enemy))
            (Components|Activation|Activate (Variables|/Game/Project/Blueprint/AI/BP_Enemy.BP_Enemy_C|GetStars _asbp_enemy) false)
            (Rendering|SetVisibility (Variables|/Game/Project/Blueprint/AI/BP_Enemy.BP_Enemy_C|GetStars _asbp_enemy) true false)
            (Niagara|SpawnSystemAttached "/Game/Project/3D/Jacopo_contetn/Lighting/lighting.lighting" (Variables|/Game/Project/Blueprint/AI/BP_Enemy.BP_Enemy_C|GetStars _asbp_enemy) "None" "0.000000,0.000000,-75.000000" "0, 0, 0" "KeepRelativeOffset" false)))
        (:CastFailed
          (bind _asbp_default_character (Utilities|Casting|CastToBP_DefaultCharacter _array_element))
          (if (not (Variables|/Game/Project/Blueprint/Player/BP_DefaultCharacter.BP_DefaultCharacter_C|GetHasShield _asbp_default_character))
            (Variables|/Script/GamelabSupermarket.DefaultCharacter|SetbIsStunned _asbp_default_character true)
            (Components|Activation|Activate (Variables|/Game/Project/Blueprint/Player/BP_DefaultCharacter.BP_DefaultCharacter_C|GetStars _asbp_default_character) false)
            (Rendering|SetVisibility (Variables|/Game/Project/Blueprint/Player/BP_DefaultCharacter.BP_DefaultCharacter_C|GetStars _asbp_default_character) true false)
            (Niagara|SpawnSystemAttached "/Game/Project/3D/Jacopo_contetn/Lighting/lighting.lighting" (Variables|/Game/Project/Blueprint/Player/BP_DefaultCharacter.BP_DefaultCharacter_C|GetStars _asbp_default_character) "None" "0.000000,0.000000,-75.000000" "0, 0, 0" "KeepRelativeOffset" false))))))
  (Variables|/Script/Engine.PrimitiveComponent|SetbGenerateOverlapEvents (Variables|Default|GetSphere) false)
  (Utilities|Time|SetTimerbyFunctionName 0 "DeStunAll" (Variables|Default|GetTime)))

(fn ConstructionScript
  (|CallParentFunction))