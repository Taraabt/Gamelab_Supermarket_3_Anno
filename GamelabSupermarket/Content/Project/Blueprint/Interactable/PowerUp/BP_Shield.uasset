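; BP_Shield is a shield power-up that grants a temporary shield to the player character or an enemy that overlaps it.
; On pickup by an unshielded target, it sets HasShield, shows the target's Shield component, then disables its sphere overlaps and hides its Niagara effect.
; A timer, fixed for the player and variable-driven for enemies, calls Destroy to remove the shield and destroy the actor.
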(event Custom|Destroy
  (bind _asbp_enemy (Utilities|Casting|CastToBP_Enemy (Variables|Default|GetShieldedEnemy))
    (:then
      (Variables|/Game/Project/Blueprint/AI/BP_Enemy.BP_Enemy_C|SetHasShield _asbp_enemy false)
      (Rendering|SetVisibility (Variables|/Game/Project/Blueprint/AI/BP_Enemy.BP_Enemy_C|GetShield _asbp_enemy) false false)
      (Actor|DestroyActor))
    (:CastFailed
      (bind _asbp_default_character (Utilities|Casting|CastToBP_DefaultCharacter (Variables|Default|GetShieldedCharacter)))
      (Variables|/Game/Project/Blueprint/Player/BP_DefaultCharacter.BP_DefaultCharacter_C|SetHasShield _asbp_default_character false)
      (Rendering|SetVisibility (Variables|/Game/Project/Blueprint/Player/BP_DefaultCharacter.BP_DefaultCharacter_C|GetShield _asbp_default_character) false false)
      (Actor|DestroyActor))))

(event EventBeginPlay
  (|CallParentFunction) ; This node is disabled and will not be called.\nDrag off pins to build functionality.
)

(event Collision|EventActorBeginOverlap
  (params (OtherActor :type Actor%20Object%20Reference))
  (|CallParentFunction 0)
  (bind _asbp_default_character (Utilities|Casting|CastToBP_DefaultCharacter OtherActor)
    (:then
      (if (not (Variables|/Game/Project/Blueprint/Player/BP_DefaultCharacter.BP_DefaultCharacter_C|GetHasShield _asbp_default_character))
        (Variables|/Game/Project/Blueprint/Player/BP_DefaultCharacter.BP_DefaultCharacter_C|SetHasShield _asbp_default_character true)
        (Rendering|SetVisibility (Variables|/Game/Project/Blueprint/Player/BP_DefaultCharacter.BP_DefaultCharacter_C|GetShield _asbp_default_character) true false)
        (Variables|Default|SetShieldedCharacter _asbp_default_character)
        (Variables|/Script/Engine.PrimitiveComponent|SetbGenerateOverlapEvents (Variables|Default|GetSphere) false)
        (Rendering|SetVisibility (Variables|Default|GetNiagara) false false)
        (Utilities|Time|SetTimerbyFunctionName 0 "Destroy" 7.0 false true)))
    (:CastFailed
      (bind _asbp_enemy (Utilities|Casting|CastToBP_Enemy OtherActor))
      (if (not (Variables|/Game/Project/Blueprint/AI/BP_Enemy.BP_Enemy_C|GetHasShield _asbp_enemy))
        (Variables|/Game/Project/Blueprint/AI/BP_Enemy.BP_Enemy_C|SetHasShield _asbp_enemy true)
        (Rendering|SetVisibility (Variables|/Game/Project/Blueprint/AI/BP_Enemy.BP_Enemy_C|GetShield _asbp_enemy) true false)
        (Variables|Default|SetShieldedEnemy _asbp_enemy)
        (Variables|/Script/Engine.PrimitiveComponent|SetbGenerateOverlapEvents (Variables|Default|GetSphere) false)
        (Rendering|SetVisibility (Variables|Default|GetNiagara) false false)
        (Utilities|Time|SetTimerbyFunctionName 0 "Destroy" (Variables|Default|GetTime) false true)))))

(event EventTick
  (params (DeltaSeconds :type Float%20%28single-precision%29))
  (|CallParentFunction DeltaSeconds) ; This node is disabled and will not be called.\nDrag off pins to build functionality.
)

(fn ConstructionScript
  (|CallParentFunction))