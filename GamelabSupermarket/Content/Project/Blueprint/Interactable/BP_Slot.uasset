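; BP_Slot is an interactable product slot that lights up as a target for either the player or a specific enemy.
; It binds to LightOn dispatchers on the player and every BP_Enemy, showing a colored plane and recording the owner.
; Interact plays a refill sound; a matching interactor clears the slot and updates its product counts.
; The slot's index returns to the GameInstance's available pool, and the interactor's interact dispatcher fires.
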(event Custom|LightOn
  (params (NewParam :type BP%20Slot%20Object%20Reference) (NewParam1 :type Color%20Structure))
  (bind _plane (Variables|Default|GetPlane))
  (Variables|Default|SetColor NewParam1)
  (if (== NewParam self)
    (Variables|Default|SetIsOn true)
    (Variables|Default|SetIsEnemy false)
    (Rendering|SetVisibility _plane true false)
    (Rendering|Material|SetColorParameterValueonMaterials _plane "color" (Math|Conversions|ToLinearColor(Color) NewParam1))))

(event Custom|LightOnEnemy
  (params (NewParam1 :type BP%20Slot%20Object%20Reference) (NewParam :type Color%20Structure) (NewParam2 :type Integer))
  (bind _plane (Variables|Default|GetPlane))
  (Variables|Default|SetColor NewParam)
  (if (== NewParam1 self)
    (Variables|Default|SetIsEnemy true)
    (Variables|Default|SetIsOn true)
    (Variables|Default|SetEnemyIndex NewParam2)
    (Rendering|SetVisibility _plane true false)
    (Rendering|Material|SetColorParameterValueonMaterials _plane "color" (Math|Conversions|ToLinearColor(Color) NewParam))))

(event EventBeginPlay
  (Variables|Default|SetEnemyIndex -1)
  (Variables|Default|SetIsOn false)
  (Rendering|SetVisibility (Variables|Default|GetPlane) false false)
  (bind _asbp_default_character (Utilities|Casting|CastToBP_DefaultCharacter (Game|Player|GetPlayerPawn 0)))
  (EventDispatchers|BindEventtoLighton _asbp_default_character (EventDispatchers|CreateEvent :!event Custom|LightOn))
  (bind _outactors (Actor|GetAllActorsOfClass "/Game/Project/Blueprint/AI/BP_Enemy.BP_Enemy_C"))
  (for _array_element _outactors
    (EventDispatchers|BindEventtoLightonEnemy _array_element (EventDispatchers|CreateEvent :!event Custom|LightOnEnemy))))

(event EventInteract
  (params (Interactor :type Character%20Object%20Reference))
  (bind _index (Variables|Default|GetIndex))
  (bind _index_2 (Variables|Default|GetIndex))
  (Audio|PlaySoundatLocation "/Game/Project/Sound/SFX/Player/Player_Mechanics/SFX_-_Refilling_Item_in_BOX.SFX_-_Refilling_Item_in_BOX" "0, 0, 0" "0, 0, 0" 0.35 1.0 0.0 0 0 0 0)
  (if (Variables|Default|GetIsOn)
    (if (not (Variables|Default|GetIsEnemy))
      (if (== Interactor (Game|Player|GetPlayerPawn 0))
        (Variables|Default|SetIsOn false)
        (Rendering|SetVisibility (Variables|Default|GetPlane) false false)
        (bind _asbp_default_character (Utilities|Casting|CastToBP_DefaultCharacter Interactor))
        (Math|Integer|IncrementInt (Variables|/Game/Project/Blueprint/Player/BP_DefaultCharacter.BP_DefaultCharacter_C|GetDeliveryProduct _asbp_default_character)
          (:%20%20
            (if (> (Utilities|Array|Length (Variables|/Game/Project/Blueprint/Player/BP_DefaultCharacter.BP_DefaultCharacter_C|GetProductName _asbp_default_character)) 0)
              (Utilities|Array|RemoveIndex (Variables|/Game/Project/Blueprint/Player/BP_DefaultCharacter.BP_DefaultCharacter_C|GetProductName _asbp_default_character) (- (Utilities|Array|Length (Variables|/Game/Project/Blueprint/Player/BP_DefaultCharacter.BP_DefaultCharacter_C|GetProductName _asbp_default_character)) 1))
              (Utilities|Array|RemoveIndex (Variables|/Game/Project/Blueprint/Player/BP_DefaultCharacter.BP_DefaultCharacter_C|GetProductSlot _asbp_default_character) (- (Utilities|Array|Length (Variables|/Game/Project/Blueprint/Player/BP_DefaultCharacter.BP_DefaultCharacter_C|GetProductName _asbp_default_character)) 1))
              (bind _asbp_game_instance (Utilities|Casting|CastToBP_GameInstance (Game|GetGameInstance)))
              (Utilities|Array|RemoveItem (Variables|/Game/Project/Blueprint/Core/BP_GameInstance.BP_GameInstance_C|GetChoose _asbp_game_instance) _index)
              (Utilities|Array|Add (Variables|/Game/Project/Blueprint/Core/BP_GameInstance.BP_GameInstance_C|GetIndexDisponibili _asbp_game_instance) _index)
              (Default|CallPlayerInteract _asbp_default_character)))))
      (else
        (bind _asbp_game_instance_2 (Utilities|Casting|CastToBP_GameInstance (Game|GetGameInstance)))
        (bind _asbp_enemy (Utilities|Casting|CastToBP_Enemy Interactor))
        (if (== _asbp_enemy (Utilities|Array|Get(acopy) (Variables|/Game/Project/Blueprint/Core/BP_GameInstance.BP_GameInstance_C|GetEnemy _asbp_game_instance_2) (- (Variables|Default|GetEnemyIndex) 1)))
          (Variables|Default|SetIsOn false)
          (Variables|Default|SetIsEnemy false)
          (Rendering|SetVisibility (Variables|Default|GetPlane) false false)
          (bind _asbp_game_instance_3 (Utilities|Casting|CastToBP_GameInstance (Game|GetGameInstance)))
          (Utilities|Array|RemoveItem (Variables|/Game/Project/Blueprint/Core/BP_GameInstance.BP_GameInstance_C|GetChoose _asbp_game_instance_3) _index_2)
          (Utilities|Array|Add (Variables|/Game/Project/Blueprint/Core/BP_GameInstance.BP_GameInstance_C|GetIndexDisponibili _asbp_game_instance_3) _index_2)
          (Variables|Default|SetEnemyIndex -1)
          (bind _result (Math|Integer|DecrementInt (Variables|/Game/Project/Blueprint/AI/BP_Enemy.BP_Enemy_C|GetNProduct _asbp_enemy))
            (:%20%20
              (Default|CallEnemyInteract _asbp_enemy (Variables|/Game/Project/Blueprint/AI/BP_Enemy.BP_Enemy_C|GetIndex _asbp_enemy) _result (Variables|/Game/Project/Blueprint/AI/BP_Enemy.BP_Enemy_C|GetDeliveryProduct _asbp_enemy)))))))))

(fn ConstructionScript)