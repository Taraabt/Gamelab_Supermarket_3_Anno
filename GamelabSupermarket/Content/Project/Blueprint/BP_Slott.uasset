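; BP_Slott is an interactable actor with a point light that toggles on and off.
; On BeginPlay it applies its Color variable, converted to a linear color, to the PointLight.
; Each Interact event flips IsOn and switches the light intensity between zero and a fixed brightness.
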(event Collision|EventActorBeginOverlap
  (params (OtherActor :type Actor%20Object%20Reference)))

(event EventTick
  (params (DeltaSeconds :type Float%20%28single-precision%29)))

(event EventInteract
  (params (Interactor :type Actor%20Object%20Reference))
  (bind _pointlight (Variables|Default|GetPointLight))
  (if (Variables|Default|GetIsOn)
    (Rendering|Components|Light|SetIntensity _pointlight 0.0)
    (Variables|Default|SetIsOn false)
    (else
      (Rendering|Components|Light|SetIntensity _pointlight 5e+03)
      (Variables|Default|SetIsOn true))))

(event EventBeginPlay
  (Rendering|Components|Light|SetLightColor (Variables|Default|GetPointLight) (Math|Conversions|ToLinearColor(Color) (Variables|Default|GetColor)) true))

(fn ConstructionScript)