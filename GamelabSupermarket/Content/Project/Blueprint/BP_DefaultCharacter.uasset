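; BP_DefaultCharacter is a player character that carries a box and can interact with objects in front of it.
; On BeginPlay it spawns a BP_Box at a mesh socket and attaches it there.
; The IA_Interact input fires a horizontal, debug-drawn Visibility line trace along the player's facing, prints the hit actor's name, and calls InteractMessage on it if it implements the Interactable interface.
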(event Collision|EventActorBeginOverlap
  (params (OtherActor :type Actor%20Object%20Reference)))

(event EventTick
  (params (DeltaSeconds :type Float%20%28single-precision%29)))

(fn ConstructionScript)

(event EventBeginPlay
  (bind _mesh (Variables|Character|GetMesh))
  (bind _socket_name (Variables|Default|GetSocket%20Name))
  (bind _returnvalue (Game|SpawnActorfromClass "/Game/Project/Blueprint/BP_Box.BP_Box_C" (Transformation|GetSocketTransform _mesh _socket_name "RTS_World") "Undefined" "MultiplyWithRoot" 0 0))
  (Transformation|AttachComponentToComponent _returnvalue _mesh _socket_name "KeepWorld" "KeepWorld" "KeepWorld" true))

(event Input|EnhancedActionEvents|EnhancedInputActionIA_Interact
  (params (ActionValue :type Boolean) (ElapsedSeconds :type Float%20%28double-precision%29) (TriggeredSeconds :type Float%20%28double-precision%29) (InputAction :type Input%20Action%20Object%20Reference :default "/Game/Project/Input/IA_Interact.IA_Interact"))
  (bind _returnvalue (Game|GetPlayerCharacter 0))
  (bind _returnvalue_2 (Transformation|GetActorLocation))
  (bind _returnvalue_3 (Transformation|GetActorTransform _returnvalue))
  (bind _returnvalue_4 (Math|Vector|GetForwardVector (.rotation _returnvalue_3)))
  (:Started
    (bind _outhit (Collision|LineTraceByChannel _returnvalue_2 (+ _returnvalue_2 (Math|Vector|MakeVector (* (.x _returnvalue_4) 2e+02) (* (.y _returnvalue_4) 2e+02) 0.0)) "TraceTypeQuery1" false 0 "ForDuration" true "(R=1.000000,G=0.000000,B=0.000000,A=1.000000)" "(R=0.000000,G=1.000000,B=0.000000,A=1.000000)" 5e+01))
    (bind _output_get (Variables|Default|SetOut%20Hit%20Hit%20Actor (.hitactor _outhit)))
    (Development|PrintString (Utilities|GetDisplayName _output_get))
    (if (Utilities|DoesObjectImplementInterface (.hitactor _outhit) "/Script/GamelabSupermarket.Interactable")
      (Class|Interactable|Interact(Message) _output_get))))