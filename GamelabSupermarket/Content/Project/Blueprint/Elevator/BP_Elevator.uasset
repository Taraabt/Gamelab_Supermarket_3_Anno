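; Elevator Blueprint that moves a Cube along the line between its StartingPoint and EndingPoint.
; StartElevator plays or reverses the ElevatorMovement timeline according to CanGoDown, interpolating the Cube's world location and setting IsMoving.
; A finished forward run clears both flags and resets a DoOnce.
; A finished reverse run passes that DoOnce, briefly waits, restores CanGoDown and automatically plays forward again.
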(event Custom|StartElevator
  (bind _endingpoint (Variables|Default|GetEndingPoint))
  (bind _returnvalue (Transformation|GetWorldLocation _endingpoint))
  (if (Variables|Default|GetCanGoDown) :!label _label
    (bind _elevatormovement (Timeline|ElevatorMovement Play)
      (:Update
        (Transformation|SetWorldLocation (Variables|Default|GetCube) (+ (* _elevatormovement (- (Transformation|GetWorldLocation (Variables|Default|GetStartingPoint)) _returnvalue)) _returnvalue) false false)
        (Variables|Default|SetIsMoving true))
      (:Finished
        (if (Variables|Default|GetCanGoDown)
          (Variables|Default|SetCanGoDown false)
          (Variables|Default|SetIsMoving false)
          (goto _label_2 Reset)
          (else
            (Utilities|FlowControl|DoOnce false :!label _label_2
              (:Completed
                (Utilities|FlowControl|Delay 0.2)
                (Variables|Default|SetCanGoDown true)
                (goto _label)))))))
    (else
      (Timeline|ElevatorMovement Reverse))))

(fn ConstructionScript)