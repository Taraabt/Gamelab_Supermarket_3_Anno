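; Player character for a timed product-shelf game, handling interaction, bumping enemies, pausing and the end screen.
; On start it draws three unique random products from DT_Product through GameInstance index pools, lights their shelves and attaches a box.
; Interact sphere-traces for Interactable actors, while Bump stuns the nearest unshielded enemy in range through its AI blackboard.
; A looping timer drives the countdown, and a debug-like input skips it to the end.
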(event Custom|Initialize
  (bind _stars (Variables|Default|GetStars))
  (bind _asbp_game_instance (Utilities|Casting|CastToBP_GameInstance (Game|GetGameInstance)))
  (for (_array_element _array_index) (Variables|/Game/Project/Blueprint/Core/BP_GameInstance.BP_GameInstance_C|GetLeaderBoard _asbp_game_instance)
    (Utilities|Array|SetArrayElem (Variables|/Game/Project/Blueprint/Core/BP_GameInstance.BP_GameInstance_C|GetLeaderBoard _asbp_game_instance) _array_index (Utilities|Struct|MakePlayer_data 0 (.name _array_element) (.colors _array_element) (.image _array_element) 0)))
  (Rendering|SetVisibility (Variables|Default|GetShield) false false)
  (Components|Activation|Deactivate _stars)
  (Rendering|SetVisibility _stars false false)
  (bind _asbp_game_instance_2 (Utilities|Casting|CastToBP_GameInstance (Game|GetGameInstance)))
  (Variables|Default|SetColor (Utilities|Array|Get(acopy) (Variables|/Game/Project/Blueprint/Core/BP_GameInstance.BP_GameInstance_C|GetColor _asbp_game_instance_2)))
  (Rendering|Material|SetColorParameterValueonMaterials (Variables|Default|GetArrowDirection) "color" (Math|Conversions|ToLinearColor(Color) (Variables|Default|GetColor)))
  (Rendering|Material|SetColorParameterValueonMaterials (Variables|Default|GetCircle) "color" (Math|Conversions|ToLinearColor(Color) (Variables|Default|GetColor)))
  (bind _outrownames (DataTable|GetDataTableRowNames "/Game/Project/Blueprint/DT_Product.DT_Product"))
  (for _index (range 0 (Utilities|Array|LastIndex _outrownames))
    (Utilities|Array|Add (Variables|/Game/Project/Blueprint/Core/BP_GameInstance.BP_GameInstance_C|GetIndexDisponibili _asbp_game_instance_2) _index))
  (for _index_2 (range 0 2)
    (bind _asbp_game_instance_3 (Utilities|Casting|CastToBP_GameInstance (Game|GetGameInstance)))
    (Variables|Default|SetRandomIndex (Math|Random|RandomIntegerinRange 0 (Utilities|Array|LastIndex (Variables|/Game/Project/Blueprint/Core/BP_GameInstance.BP_GameInstance_C|GetIndexDisponibili _asbp_game_instance_3))))
    (Utilities|Array|Add (Variables|/Game/Project/Blueprint/Core/BP_GameInstance.BP_GameInstance_C|GetChoose _asbp_game_instance_3) (Utilities|Array|Get(acopy) (Variables|/Game/Project/Blueprint/Core/BP_GameInstance.BP_GameInstance_C|GetIndexDisponibili _asbp_game_instance_3) (Variables|Default|GetRandomIndex)))
    (bind _outrownames_2 (DataTable|GetDataTableRowNames "/Game/Project/Blueprint/DT_Product.DT_Product"))
    (bind _returnvalue (Utilities|GetDataTableRow "/Game/Project/Blueprint/DT_Product.DT_Product" (Utilities|Array|Get(acopy) _outrownames_2 (Utilities|Array|Get(acopy) (Variables|/Game/Project/Blueprint/Core/BP_GameInstance.BP_GameInstance_C|GetIndexDisponibili _asbp_game_instance_3) (Variables|Default|GetRandomIndex))))
      (:then
        (Utilities|Array|RemoveItem (Variables|/Game/Project/Blueprint/Core/BP_GameInstance.BP_GameInstance_C|GetIndexDisponibili _asbp_game_instance_3) (Utilities|Array|Get(acopy) (Variables|/Game/Project/Blueprint/Core/BP_GameInstance.BP_GameInstance_C|GetIndexDisponibili _asbp_game_instance_3) (Variables|Default|GetRandomIndex)))
        (Utilities|Array|Add (Variables|Default|GetProductName) (.ProductName (Utilities|Struct|BreakStructDatatable _returnvalue)))
        (Utilities|Array|Add (Variables|Default|GetProductSlot) (Utilities|String|ToString(Integer) (.Shelf (Utilities|Struct|BreakStructDatatable _returnvalue)))))))
  (CallFunction|ActivateShelf))

(event Custom|UpdateUI
  (bind _returnvalue (Game|GetPlayerController 0))
  (bind _time (Variables|Default|GetTime))
  (bind _time_2 (Variables|Default|GetTime))
  (Math|Float|DecrementFloat _time_2
    (:%20%20
      (if (== _time_2 0.0)
        (Default|CallUpdateTimer _time)
        (Game|SetGamePaused true)
        (bind _returnvalue_2 (Game|ConstructObjectfromClass "/Game/Project/UI/WBP_EndScreen.WBP_EndScreen_C"))
        (UserInterface|Viewport|AddtoViewport _returnvalue_2 0)
        (Input|DisableInput _returnvalue)
        (Variables|/Script/Engine.PlayerController|SetbShowMouseCursor _returnvalue true)
        (else
          (Default|CallUpdateTimer _time))))))

(event Custom|DeStunned
  (bind _closerenemy (Variables|Default|GetCloserEnemy))
  (bind _stars (Variables|/Game/Project/Blueprint/AI/BP_Enemy.BP_Enemy_C|GetStars _closerenemy))
  (bind _output_get (Variables|/Game/Project/Blueprint/AI/BP_Enemy.BP_Enemy_C|SetIsStunned _closerenemy false))
  (AI|Components|Blackboard|SetValueasBool (Variables|/Script/AIModule.AIController|GetBlackboard (AI|GetAIController _closerenemy)) (Variables|Default|GetStunned) _output_get)
  (Variables|Default|SetCanBump true)
  (Components|Activation|Deactivate _stars)
  (Rendering|SetVisibility _stars false false))

(event Custom|UpdateBumpBar
  (if (not (Variables|Default|GetCanBump))
    (Default|CallUpdateBump (Variables|Default|GetBumpTimer))))

(event Custom|AddProduct
  (bind _asbp_game_instance (Utilities|Casting|CastToBP_GameInstance (Game|GetGameInstance)))
  (bind _outrownames (DataTable|GetDataTableRowNames "/Game/Project/Blueprint/DT_Product.DT_Product"))
  (Variables|Default|SetRandomIndex (Math|Random|RandomIntegerinRange 0 (Utilities|Array|LastIndex (Variables|/Game/Project/Blueprint/Core/BP_GameInstance.BP_GameInstance_C|GetIndexDisponibili _asbp_game_instance))))
  (bind _returnvalue (Utilities|GetDataTableRow "/Game/Project/Blueprint/DT_Product.DT_Product" (Utilities|Array|Get(acopy) _outrownames (Utilities|Array|Get(acopy) (Variables|/Game/Project/Blueprint/Core/BP_GameInstance.BP_GameInstance_C|GetIndexDisponibili _asbp_game_instance) (Variables|Default|GetRandomIndex))))
    (:then
      (Utilities|Array|Add (Variables|Default|GetProductName) (.productname _returnvalue))
      (Utilities|Array|Add (Variables|Default|GetProductSlot) (Utilities|String|ToString(Integer) (.shelf _returnvalue)))
      (bind _asbp_game_instance_2 (Utilities|Casting|CastToBP_GameInstance (Game|GetGameInstance)))
      (bind _returnvalue_2 (Utilities|Array|Add (Variables|/Game/Project/Blueprint/Core/BP_GameInstance.BP_GameInstance_C|GetChoose _asbp_game_instance_2) (Utilities|Array|Get(acopy) (Variables|/Game/Project/Blueprint/Core/BP_GameInstance.BP_GameInstance_C|GetIndexDisponibili _asbp_game_instance_2) (Variables|Default|GetRandomIndex))))
      (Utilities|Array|RemoveItem (Variables|/Game/Project/Blueprint/Core/BP_GameInstance.BP_GameInstance_C|GetIndexDisponibili _asbp_game_instance_2) (Utilities|Array|Get(acopy) (Variables|/Game/Project/Blueprint/Core/BP_GameInstance.BP_GameInstance_C|GetChoose _asbp_game_instance_2) _returnvalue_2))
      (Default|CallLighton (Utilities|Array|Get(acopy) (Variables|Default|GetSlot) (Utilities|Array|Get(acopy) (Variables|/Game/Project/Blueprint/Core/BP_GameInstance.BP_GameInstance_C|GetChoose _asbp_game_instance_2) _returnvalue_2)) (Variables|Default|GetColor)))))

(event Custom|PlaceBox
  (bind _mesh (Variables|Character|GetMesh))
  (bind _socket_name (Variables|Default|GetSocket%20Name))
  (bind _returnvalue (Game|SpawnActorfromClass "/Game/Project/Blueprint/Player/BP_Box.BP_Box_C" (Transformation|GetSocketTransform _mesh _socket_name "RTS_World") "Undefined" "MultiplyWithRoot" 0 0))
  (Transformation|AttachComponentToComponent _returnvalue _mesh _socket_name "KeepWorld" "KeepWorld" "KeepWorld" true)
  (Utilities|Time|SetTimerbyFunctionName 0 "UpdateUI" 1.0 true))

(event Custom|ActivateShelf
  (bind _asbp_game_instance (Utilities|Casting|CastToBP_GameInstance (Game|GetGameInstance)))
  (for _index (range 0 2)
    (Default|CallLighton (Utilities|Array|Get(acopy) (Variables|Default|GetSlot) (Utilities|Array|Get(acopy) (Variables|/Game/Project/Blueprint/Core/BP_GameInstance.BP_GameInstance_C|GetChoose _asbp_game_instance) _index)) (Variables|Default|GetColor)))
  (CallFunction|PlaceBox))

(event Input|EnhancedActionEvents|EnhancedInputActionIA_Bump
  (params (ActionValue :type Boolean) (ElapsedSeconds :type Float%20%28double-precision%29) (TriggeredSeconds :type Float%20%28double-precision%29) (InputAction :type Input%20Action%20Object%20Reference :default "/Game/Project/Input/IA/IA_Bump.IA_Bump"))
  (:Started
    (if (not (Variables|Default|GetbIsStunned))
      (if (Variables|Default|GetCanBump)
        (Niagara|SpawnSystemAttached "/Game/Project/3D/Knife_light/VFX/NE_attack01.NE_attack01" (Variables|Character|GetMesh) "thigh_r" "0, 0, 0" "0.000000,0.000000,-90.000000" "KeepRelativeOffset" true)
        (Audio|PlaySoundatLocation "/Game/Project/Sound/SFX/Player/Player_Mechanics/SFX_-_Bump_.SFX_-_Bump_" "0, 0, 0" "0, 0, 0" 1.0 1.0 0.0 0 0 0 0)
        (CallFunction|Bump)
        (Utilities|Time|SetTimerbyFunctionName 0 "UpdateBumpBar" 0.1 true true)))))

(event Input|EnhancedActionEvents|EnhancedInputActionIA_Move
  (params (ActionValue :type Vector%202D%20Structure) (ElapsedSeconds :type Float%20%28double-precision%29) (TriggeredSeconds :type Float%20%28double-precision%29) (InputAction :type Input%20Action%20Object%20Reference :default "/Game/Project/Input/IA/IA_Move.IA_Move"))
  (bind _niagara (Variables|Default|GetNiagara))
  (:Started
    (if (not (Variables|Default|GetbIsStunned))
      (Components|Activation|SetActive _niagara true false)))
  (:Completed
    (if (not (Variables|Default|GetbIsStunned))
      (Components|Activation|SetActive _niagara false false))))

(event Input|EnhancedActionEvents|EnhancedInputActionIA_Interact
  (params (ActionValue :type Boolean) (ElapsedSeconds :type Float%20%28double-precision%29) (TriggeredSeconds :type Float%20%28double-precision%29) (InputAction :type Input%20Action%20Object%20Reference :default "/Game/Project/Input/IA/IA_Interact.IA_Interact"))
  (bind _returnvalue (Transformation|GetActorLocation))
  (bind _returnvalue_2 (Game|GetPlayerCharacter 0))
  (bind _returnvalue_3 (Transformation|GetActorTransform _returnvalue_2))
  (bind _returnvalue_4 (Math|Vector|GetForwardVector (.rotation _returnvalue_3)))
  (:Started
    (if (not (Variables|Default|GetbIsStunned))
      (bind _outhit (Collision|SphereTraceByChannel _returnvalue (+ _returnvalue (Math|Vector|MakeVector (* (.x _returnvalue_4) 2e+02) (* (.y _returnvalue_4) 2e+02) 0.0)) 4e+01 "TraceTypeQuery1" false 0 "None" true "(R=1.000000,G=0.000000,B=0.000000,A=1.000000)" "(R=0.000000,G=1.000000,B=0.000000,A=1.000000)" 2e+01))
      (if (Utilities|DoesObjectImplementInterface (.hitactor _outhit) "/Script/GamelabSupermarket.Interactable")
        (Class|Interactable|Interact(Message) (.hitactor _outhit) self)
        (Default|CallPlayerInteract)))))

(event Input|EnhancedActionEvents|EnhancedInputActionIA_MenuPause
  (params (ActionValue :type Boolean) (ElapsedSeconds :type Float%20%28double-precision%29) (TriggeredSeconds :type Float%20%28double-precision%29) (InputAction :type Input%20Action%20Object%20Reference :default "/Game/Project/Input/IA/IA_MenuPause.IA_MenuPause"))
  (:Started
    (if (not (Variables|Default|GetIsPaused))
      (Variables|Default|SetIsPaused true)
      (bind _returnvalue (Game|ConstructObjectfromClass "/Game/Project/UI/WBP_MenuPause.WBP_MenuPause_C"))
      (bind _output_get (Variables|Default|SetPauseMenuWidget _returnvalue))
      (UserInterface|Viewport|AddtoViewport _output_get 0)
      (Input|SetInputModeGameandUI (Game|GetPlayerController 0) _output_get "DoNotLock" true false)
      (Variables|/Script/Engine.PlayerController|SetbShowMouseCursor (Game|GetPlayerController 0) true)
      (Game|SetGamePaused true)
      (else
        (Variables|Default|SetIsPaused false)
        (Widget|RemovefromParent (Variables|Default|GetPauseMenuWidget))
        (Variables|/Script/Engine.PlayerController|SetbShowMouseCursor (Game|GetPlayerController 0) false)
        (Game|SetGamePaused false)
        (Input|SetInputModeGameOnly (Game|GetPlayerController 0) false)))))

(event Input|EnhancedActionEvents|EnhancedInputActionAvengers_Endgame
  (params (ActionValue :type Boolean) (ElapsedSeconds :type Float%20%28double-precision%29) (TriggeredSeconds :type Float%20%28double-precision%29) (InputAction :type Input%20Action%20Object%20Reference :default "/Game/Project/Input/IA/Avengers_Endgame.Avengers_Endgame"))
  (Variables|Default|SetTime 1.0))

(event EventBeginPlay
  (CallFunction|Initialize)
  (Components|Activation|SetActive (Variables|Default|GetNiagara) false false))

(fn ConstructionScript)

(fn Bump
  (LocalVariables|SetMinDistance 99999.0)
  (Variables|Default|SetCanBump false)
  (bind _outactors (Actor|GetAllActorsOfClass "/Script/Engine.Character"))
  (for _array_element _outactors
    (bind _asbp_enemy (Utilities|Casting|CastToBP_Enemy _array_element))
    (if (< (Transformation|GetDistanceTo _array_element) (LocalVariables|GetMinDistance))
      (LocalVariables|SetMinDistance (Transformation|GetDistanceTo _array_element))
      (Variables|Default|SetCloserEnemy _asbp_enemy)))
  (if (<= (LocalVariables|GetMinDistance) 3e+02)
    (if (not (Variables|/Game/Project/Blueprint/AI/BP_Enemy.BP_Enemy_C|GetHasShield (Variables|Default|GetCloserEnemy)))
      (bind _output_get (Variables|/Game/Project/Blueprint/AI/BP_Enemy.BP_Enemy_C|SetIsStunned (Variables|Default|GetCloserEnemy) true))
      (AI|Components|Blackboard|SetValueasBool (Variables|/Script/AIModule.AIController|GetBlackboard (AI|GetAIController (Variables|Default|GetCloserEnemy))) (Variables|Default|GetStunned) _output_get)
      (Components|Movement|StopMovementImmediately (Variables|/Script/Engine.Character|GetCharacterMovement (Variables|Default|GetCloserEnemy)))
      (Components|Activation|Activate (Variables|/Game/Project/Blueprint/AI/BP_Enemy.BP_Enemy_C|GetStars (Variables|Default|GetCloserEnemy)) false)
      (Rendering|SetVisibility (Variables|/Game/Project/Blueprint/AI/BP_Enemy.BP_Enemy_C|GetStars (Variables|Default|GetCloserEnemy)) true false)
      (Default|DeActiveSmoke (Variables|Default|GetCloserEnemy)))))