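; BP_Enemy is an AI rival that competes with the player at stocking shelves.
; It claims random DT_Product entries from the GameInstance's shared pool, lights matching slots in its color and carries a box.
; Search events write its slot and warehouse targets to the Blackboard.
; AI perception triggers Bump, stunning the nearest unshielded character in range; the Stun event also bumps, then schedules the stun's release.
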(event OnTargetPerceptionUpdated(AIPerception)
  (params (Actor :type Actor%20Object%20Reference) (Stimulus :type AI%20Stimulus%20Structure))
  (Utilities|FlowControl|Delay 0.2)
  (Utilities|Casting|CastToCharacter Actor)
  (if (Variables|Default|GetCan%20Bump)
    (if (not (Variables|Default|GetIsStunned))
      (Niagara|SpawnSystemAttached "/Game/Project/3D/Knife_light/VFX/NE_attack01.NE_attack01" (Variables|Character|GetMesh) "thigh_r" "0, 0, 0" "0.000000,0.000000,-90.000000" "KeepRelativeOffset" true)
      (Audio|PlaySoundatLocation "/Game/Project/Sound/SFX/Player/Player_Mechanics/SFX_-_Bump_.SFX_-_Bump_" "0, 0, 0" "0, 0, 0" 1.0 1.0 0.0 0 0 0 0)
      (CallFunction|Bump)
      (bind _returnvalue (Utilities|Time|SetTimerbyFunctionName 0 "UpdateBumpBar" 0.1 true))
      (Variables|Default|SetNewVar _returnvalue))))

(event Custom|Initialize
  (bind _stars (Variables|Default|GetStars))
  (Rendering|SetVisibility (Variables|Default|GetShield) false false)
  (Components|Activation|Deactivate _stars)
  (Rendering|SetVisibility _stars false false)
  (Variables|Default|SetToStock (Math|Random|RandomIntegerinRange 1 3))
  (bind _asbp_game_instance (Utilities|Casting|CastToBP_GameInstance (Game|GetGameInstance)))
  (Variables|Default|SetColor (Utilities|Array|Get(acopy) (Variables|/Game/Project/Blueprint/Core/BP_GameInstance.BP_GameInstance_C|GetColor _asbp_game_instance) (Variables|Default|GetIndex)))
  (for _index (range 0 2)
    (bind _asbp_game_instance_2 (Utilities|Casting|CastToBP_GameInstance (Game|GetGameInstance)))
    (Variables|Default|SetRandomIndex (Math|Random|RandomIntegerinRange 0 (Utilities|Array|LastIndex (Variables|/Game/Project/Blueprint/Core/BP_GameInstance.BP_GameInstance_C|GetIndexDisponibili _asbp_game_instance_2))))
    (Utilities|Array|Add (Variables|/Game/Project/Blueprint/Core/BP_GameInstance.BP_GameInstance_C|GetChoose _asbp_game_instance_2) (Utilities|Array|Get(acopy) (Variables|/Game/Project/Blueprint/Core/BP_GameInstance.BP_GameInstance_C|GetIndexDisponibili _asbp_game_instance_2) (Variables|Default|GetRandomIndex)))
    (bind _outrownames (DataTable|GetDataTableRowNames "/Game/Project/Blueprint/DT_Product.DT_Product"))
    (bind _returnvalue (Utilities|GetDataTableRow "/Game/Project/Blueprint/DT_Product.DT_Product" (Utilities|Array|Get(acopy) _outrownames (Utilities|Array|Get(acopy) (Variables|/Game/Project/Blueprint/Core/BP_GameInstance.BP_GameInstance_C|GetIndexDisponibili _asbp_game_instance_2) (Variables|Default|GetRandomIndex))))
      (:then
        (Utilities|Array|RemoveItem (Variables|/Game/Project/Blueprint/Core/BP_GameInstance.BP_GameInstance_C|GetIndexDisponibili _asbp_game_instance_2) (Utilities|Array|Get(acopy) (Variables|/Game/Project/Blueprint/Core/BP_GameInstance.BP_GameInstance_C|GetIndexDisponibili _asbp_game_instance_2) (Variables|Default|GetRandomIndex)))
        (Utilities|Array|Add (Variables|Default|GetProductName) (.ProductName (Utilities|Struct|BreakStructDatatable _returnvalue)))
        (Utilities|Array|Add (Variables|Default|GetProductSlot) (Utilities|String|ToString(Integer) (.Shelf (Utilities|Struct|BreakStructDatatable _returnvalue)))))))
  (CallFunction|ActivateShelf))

(event Custom|ActiveNiagara
  (Components|Activation|SetActive (Variables|Default|GetNiagara) true false))

(event Custom|ActivateShelf
  (bind _asbp_game_instance (Utilities|Casting|CastToBP_GameInstance (Game|GetGameInstance)))
  (for _index (range 0 2)
    (bind _asbp_default_character (Utilities|Casting|CastToBP_DefaultCharacter (Game|Player|GetPlayerPawn 0)))
    (Math|Integer|IncrementInt (Variables|Default|GetNProduct)
      (:%20%20
        (Default|CallLightonEnemy (Utilities|Array|Get(acopy) (Variables|/Game/Project/Blueprint/Player/BP_DefaultCharacter.BP_DefaultCharacter_C|GetSlot _asbp_default_character) (Utilities|Array|Get(acopy) (Variables|/Game/Project/Blueprint/Core/BP_GameInstance.BP_GameInstance_C|GetChoose _asbp_game_instance) (+ _index (* (Variables|Default|GetIndex) 3)))) (Variables|Default|GetColor) (Variables|Default|GetIndex)))))
  (CallFunction|PlaceBox))

(event Custom|DeStunned
  (bind _closerenemy (Variables|Default|GetCloserEnemy))
  (Utilities|Time|ClearandInvalidateTimerbyHandle (Variables|Default|GetNewVar))
  (bind _asbp_enemy (Utilities|Casting|CastToBP_Enemy _closerenemy)
    (:then
      (bind _output_get (Variables|BP_Enemy_C|SetIsStunned _asbp_enemy false))
      (AI|Components|Blackboard|SetValueasBool (Variables|/Script/AIModule.AIController|GetBlackboard (AI|GetAIController _asbp_enemy)) (Variables|Default|GetStunned) _output_get)
      (Components|Activation|Deactivate (Variables|BP_Enemy_C|GetStars _asbp_enemy))
      (Rendering|SetVisibility (Variables|BP_Enemy_C|GetStars _asbp_enemy) false false)
      (Variables|Default|SetCan%20Bump true))
    (:CastFailed
      (bind _asbp_default_character (Utilities|Casting|CastToBP_DefaultCharacter _closerenemy))
      (Variables|/Script/GamelabSupermarket.DefaultCharacter|SetbIsStunned _asbp_default_character false)
      (Components|Activation|Deactivate (Variables|/Game/Project/Blueprint/Player/BP_DefaultCharacter.BP_DefaultCharacter_C|GetStars _asbp_default_character))
      (Rendering|SetVisibility (Variables|/Game/Project/Blueprint/Player/BP_DefaultCharacter.BP_DefaultCharacter_C|GetStars _asbp_default_character) false false)
      (Variables|Default|SetCan%20Bump true))))

(event Custom|UpdateBumpBar
  (if (not (Variables|Default|GetCan%20Bump))
    (Default|CallEnemyBump (Variables|Default|GetIndex) (Variables|Default|GetBumpTimer))))

(event Custom|AddProduct
  (bind _nproduct (Variables|Default|GetNProduct))
  (bind _asbp_game_instance (Utilities|Casting|CastToBP_GameInstance (Game|GetGameInstance)))
  (bind _outrownames (DataTable|GetDataTableRowNames "/Game/Project/Blueprint/DT_Product.DT_Product"))
  (Variables|Default|SetRandomIndex (Math|Random|RandomIntegerinRange 0 (Utilities|Array|LastIndex (Variables|/Game/Project/Blueprint/Core/BP_GameInstance.BP_GameInstance_C|GetIndexDisponibili _asbp_game_instance))))
  (bind _returnvalue (Utilities|GetDataTableRow "/Game/Project/Blueprint/DT_Product.DT_Product" (Utilities|Array|Get(acopy) _outrownames (Utilities|Array|Get(acopy) (Variables|/Game/Project/Blueprint/Core/BP_GameInstance.BP_GameInstance_C|GetIndexDisponibili _asbp_game_instance) (Variables|Default|GetRandomIndex))))
    (:then
      (Utilities|Array|Add (Variables|Default|GetProductName) (.productname _returnvalue))
      (Utilities|Array|Add (Variables|Default|GetProductSlot) (Utilities|String|ToString(Integer) (.shelf _returnvalue)))
      (bind _asbp_game_instance_2 (Utilities|Casting|CastToBP_GameInstance (Game|GetGameInstance)))
      (bind _returnvalue_2 (Utilities|Array|Add (Variables|/Game/Project/Blueprint/Core/BP_GameInstance.BP_GameInstance_C|GetChoose _asbp_game_instance_2) (Utilities|Array|Get(acopy) (Variables|/Game/Project/Blueprint/Core/BP_GameInstance.BP_GameInstance_C|GetIndexDisponibili _asbp_game_instance_2) (Variables|Default|GetRandomIndex))))
      (bind _asbp_default_character (Utilities|Casting|CastToBP_DefaultCharacter (Game|Player|GetPlayerPawn 0)))
      (Utilities|Array|RemoveItem (Variables|/Game/Project/Blueprint/Core/BP_GameInstance.BP_GameInstance_C|GetIndexDisponibili _asbp_game_instance_2) (Utilities|Array|Get(acopy) (Variables|/Game/Project/Blueprint/Core/BP_GameInstance.BP_GameInstance_C|GetChoose _asbp_game_instance_2) _returnvalue_2))
      (Math|Integer|IncrementInt _nproduct
        (:%20%20
          (Default|CallLightonEnemy (Utilities|Array|Get(acopy) (Variables|/Game/Project/Blueprint/Player/BP_DefaultCharacter.BP_DefaultCharacter_C|GetSlot _asbp_default_character) (Utilities|Array|Get(acopy) (Variables|/Game/Project/Blueprint/Core/BP_GameInstance.BP_GameInstance_C|GetChoose _asbp_game_instance_2) _returnvalue_2)) (Variables|Default|GetColor) (Variables|Default|GetIndex))
          (Default|CallEnemyInteract (Variables|Default|GetIndex) _nproduct (Variables|Default|GetDeliveryProduct))
          (if (< (Variables|Default|GetNProduct) 3)
            (CallFunction|AddProduct)))))))

(event Custom|PlaceBox
  (bind _mesh (Variables|Character|GetMesh))
  (bind _handsocket (Variables|Default|GetHandSocket))
  (bind _returnvalue (Game|SpawnActorfromClass "/Game/Project/Blueprint/Player/BP_Box.BP_Box_C" (Transformation|GetSocketTransform _mesh _handsocket "RTS_World") "Undefined" "MultiplyWithRoot" 0 0))
  (Transformation|AttachComponentToComponent _returnvalue _mesh _handsocket "KeepWorld" "KeepWorld" "KeepWorld" true))

(event Custom|SearchNearest
  (bind _asbp_default_character (Utilities|Casting|CastToBP_DefaultCharacter (Game|Player|GetPlayerPawn 0)))
  (bind _array_element (Utilities|Array|ForEachLoopwithBreak (Variables|/Game/Project/Blueprint/Player/BP_DefaultCharacter.BP_DefaultCharacter_C|GetSlot _asbp_default_character) :!label _label)
    (:LoopBody
      (if (== (Variables|Default|GetIndex) (Variables|/Game/Project/Blueprint/Interactable/BP_Slot.BP_Slot_C|GetEnemyIndex _array_element))
        (bind _asaic_player_aicontroller (Utilities|Casting|CastToAIC_PlayerAIController (AI|GetAIController self)))
        (AI|Components|Blackboard|SetValueasObject (Variables|/Script/AIModule.AIController|GetBlackboard _asaic_player_aicontroller) (Variables|Default|GetSlotToSearch) _array_element)
        (goto _label Break)))))

(event Custom|DeActiveSmoke
  (Components|Activation|SetActive (Variables|Default|GetNiagara) false false))

(event Custom|SearchWarehouse
  (bind _outactors (Actor|GetAllActorsOfClass "/Game/Project/Blueprint/Interactable/BP_Warehouse.BP_Warehouse_C"))
  (for _array_element _outactors
    (if (== (Variables|Default|GetIndex) (Variables|/Game/Project/Blueprint/Interactable/BP_Warehouse.BP_Warehouse_C|GetIndex _array_element))
      (bind _asaic_player_aicontroller (Utilities|Casting|CastToAIC_PlayerAIController (AI|GetAIController self)))
      (AI|Components|Blackboard|SetValueasObject (Variables|/Script/AIModule.AIController|GetBlackboard _asaic_player_aicontroller) (Variables|Default|GetMyWarehouse) _array_element))))

(event Custom|Stun
  (CallFunction|Bump)
  (Utilities|Time|SetTimerbyFunctionName 0 "DeStunned" 3.0))

(event EventBeginPlay
  (bind _color (Variables|Default|GetColor))
  (Utilities|FlowControl|Delay 0.2)
  (Components|Activation|SetActive (Variables|Default|GetNiagara) false false)
  (Rendering|Material|SetMaterial (Variables|Character|GetMesh) 0 (Variables|Default|GetMaterial))
  (Rendering|Material|SetColorParameterValueonMaterials (Variables|Default|GetArrowDirection) "color" (Math|Conversions|ToLinearColor(Color) _color))
  (Rendering|Material|SetColorParameterValueonMaterials (Variables|Default|GetCircle) "color" (Math|Conversions|ToLinearColor(Color) _color))
  (CallFunction|Initialize))

(fn ConstructionScript)

(fn Bump
  (LocalVariables|SetMinDistance 99999.0)
  (Variables|Default|SetCan%20Bump false)
  (bind _outactors (Actor|GetAllActorsOfClass "/Script/Engine.Character"))
  (for _array_element _outactors
    (if (!= self _array_element)
      (bind _asbp_enemy (Utilities|Casting|CastToBP_Enemy _array_element)
        (:then
          (if (< (Transformation|GetDistanceTo _asbp_enemy) (LocalVariables|GetMinDistance))
            (LocalVariables|SetMinDistance (Transformation|GetDistanceTo _asbp_enemy))
            (Variables|Default|SetCloserEnemy _asbp_enemy)))
        (:CastFailed
          (bind _asbp_default_character (Utilities|Casting|CastToBP_DefaultCharacter _array_element))
          (if (< (Transformation|GetDistanceTo _asbp_default_character) (LocalVariables|GetMinDistance))
            (LocalVariables|SetMinDistance (Transformation|GetDistanceTo _asbp_enemy))
            (Variables|Default|SetCloserEnemy _asbp_default_character))))))
  (if (<= (LocalVariables|GetMinDistance) 3e+02)
    (bind _asbp_enemy_2 (Utilities|Casting|CastToBP_Enemy (Variables|Default|GetCloserEnemy))
      (:then
        (if (not (Variables|BP_Enemy_C|GetHasShield _asbp_enemy_2))
          (bind _output_get (Variables|BP_Enemy_C|SetIsStunned _asbp_enemy_2 true))
          (AI|Components|Blackboard|SetValueasBool (Variables|/Script/AIModule.AIController|GetBlackboard (AI|GetAIController _asbp_enemy_2)) (Variables|Default|GetStunned) _output_get)
          (Components|Activation|Activate (Variables|BP_Enemy_C|GetStars _asbp_enemy_2) false)
          (Rendering|SetVisibility (Variables|BP_Enemy_C|GetStars _asbp_enemy_2) true false)
          (Components|Movement|StopMovementImmediately (Variables|/Script/Engine.Character|GetCharacterMovement _asbp_enemy_2))
          (CallFunction|DeActiveSmoke _asbp_enemy_2)))
      (:CastFailed
        (bind _asbp_default_character_2 (Utilities|Casting|CastToBP_DefaultCharacter (Variables|Default|GetCloserEnemy)))
        (if (not (Variables|/Game/Project/Blueprint/Player/BP_DefaultCharacter.BP_DefaultCharacter_C|GetHasShield _asbp_default_character_2))
          (Variables|/Script/GamelabSupermarket.DefaultCharacter|SetbIsStunned _asbp_default_character_2 true)
          (Components|Activation|Activate (Variables|/Game/Project/Blueprint/Player/BP_DefaultCharacter.BP_DefaultCharacter_C|GetStars _asbp_default_character_2) false)
          (Rendering|SetVisibility (Variables|/Game/Project/Blueprint/Player/BP_DefaultCharacter.BP_DefaultCharacter_C|GetStars _asbp_default_character_2) true false)
          (Components|Movement|StopMovementImmediately (Variables|/Script/Engine.Character|GetCharacterMovement _asbp_default_character_2)))))))